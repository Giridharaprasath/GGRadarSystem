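; Base actor for secrets that a radar can detect through a highlight radius sphere.
; The construction script sizes the sphere from a radius variable.
; When another actor begins or ends overlap, it looks for that actor's BP_RadarComponent and, if one exists, notifies it of entering or leaving secret range, passing itself as the source.
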(event `self.Highlight Radius.OnComponentBeginOverlap`
  (params (OverlappedComponent :type "PrimitiveComponent Object Reference") (OtherActor :type "Actor Object Reference") (OtherComp :type "PrimitiveComponent Object Reference") (OtherBodyIndex :type Integer) (bFromSweep :type Boolean) (SweepResult :type "HitResult Structure (by ref)"))
  (bind _returnvalue (`self.GetComponentByClass` OtherActor "/GGRadarSystem/Components/BP_RadarComponent.BP_RadarComponent_C"))
  (`/Engine/EditorBlueprintResources/StandardMacros.IsValid` _returnvalue
    (:`Is Valid`
      (`/GGRadarSystem/Components/BP_RadarComponent.On Enter Secret Range` _returnvalue self))))

(event `self.Highlight Radius.OnComponentEndOverlap`
  (params (OverlappedComponent :type "PrimitiveComponent Object Reference") (OtherActor :type "Actor Object Reference") (OtherComp :type "PrimitiveComponent Object Reference") (OtherBodyIndex :type Integer))
  (bind _returnvalue (`self.GetComponentByClass` OtherActor "/GGRadarSystem/Components/BP_RadarComponent.BP_RadarComponent_C"))
  (`/Engine/EditorBlueprintResources/StandardMacros.IsValid` _returnvalue
    (:`Is Valid`
      (`/GGRadarSystem/Components/BP_RadarComponent.On Leave Secret Range` _returnvalue self))))

(fn `UserConstructionScript`
  (`SphereComponent.SetSphereRadius` (`self.Highlight Radius`) (`self.HighlightRadius`) true))