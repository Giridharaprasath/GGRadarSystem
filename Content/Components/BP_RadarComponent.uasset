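; Player component that drives a horizontal compass-style radar HUD showing directions, landmarks and quest markers.
; It creates WBP_Radar and gathers landmark actors; turn and move events refresh widget positions, marker distances and elevation arrows while visible.
; Shortest yaw difference from the camera maps 90 degrees either side to horizontal translation, optionally pinning off-sight markers to the edges.
; It also manages the main quest marker, animated show/hide and nearby-secret highlighting.
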(event `Initialize Radar`
  (params (Player :type "Actor Object Reference") (Camera :type "CameraComponent Object Reference"))
  ;[0 0 0] Initialize Radar
  (set `self.Player Reference` Player)
  (set `self.Camera Reference` Camera)
  (bind _returnvalue (`|CreateWidget` "/GGRadarSystem/UIs/WBP_Radar.WBP_Radar_C"))
  (set `self.WBP Radar` _returnvalue)
  (`self.Add Directions`)
  (`self.Add Landmarks`)
  (`UserWidget.AddToViewport` (`self.WBP Radar`) 0)
  (`self.On Player Turned`)
  (`self.On Player Moved`))

(event `Set Radar Visibility`
  (params (`Show Radar` :type Boolean) (`Use Animation` :type Boolean))
  (bind _wbp_radar (`self.WBP Radar`))
  (bind _wbp_radar_2 (`self.WBP Radar`))
  (bind _radarblendanim (`/GGRadarSystem/UIs/WBP_Radar.RadarBlendAnim` _wbp_radar_2))
  (bind _radarblendanim_2 (`/GGRadarSystem/UIs/WBP_Radar.RadarBlendAnim` _wbp_radar))
  (if (and (!= `Show Radar` (`self.bIs Visible`)) (`self.bCan Change Visibility`))
    (set `self.bCan Change Visibility` false)
    (set `self.bIs Visible` `Show Radar`)
    (`self.On Player Turned`)
    (`self.On Player Moved`)
    (if `Use Animation`
      (if (`self.bIs Visible`)
        ;[0 0 0] Play Fade In Animation
        (`Widget.SetVisibility` _wbp_radar "SelfHitTestInvisible")
        (`UserWidget.PlayAnimation` _wbp_radar _radarblendanim_2 0.0 1 "Reverse" 1.0 false)
        (`KismetSystemLibrary.Delay` (`WidgetAnimation.GetEndTime` _radarblendanim_2))
        (set `self.bCan Change Visibility` true)
        (else
          ;[0 0 0] Play Fade Out Animation
          (`UserWidget.PlayAnimation` _wbp_radar_2 _radarblendanim 0.0 1 "Forward" 1.0 false)
          (`KismetSystemLibrary.Delay` (`WidgetAnimation.GetEndTime` _radarblendanim))
          (`Widget.SetVisibility` (`self.WBP Radar`) "Hidden")
          (set `self.bCan Change Visibility` true)))
      (else
        ;[0 0 0] Show or Hide Radar without Animation
        (`Widget.SetVisibility` (`self.WBP Radar`) (select `bool` (`self.bIs Visible`) :`false` "Hidden" :`true` "SelfHitTestInvisible" :!type "ESlateVisibility Enum"))
        (set `self.bCan Change Visibility` true)))))

(event `On Player Turned`
  ;[0 0 0] Event On Player Turned
  (if (`self.bIs Visible`)
    (`self.Update Direction Widgets`)
    (`self.Update Marker Positions`)
    (`self.Update Landmark Positions`)))

(event `On Player Moved`
  ;[0 0 0] Event On Player Moved
  (if (`self.bIs Visible`)
    (`self.Update Marker Distances`)
    (`self.Update Marker Positions`)
    (`self.Update Landmark Positions`)
    (`self.Update Marker Elevations`)))

(event `On Enter Secret Range`
  (params (Secret :type "/GGRadarSystem/Actors/AC_HighlightRadar_Base Object Reference"))
  ;[0 0 0] Event On Player Entered Secret Range
  (if (not (`KismetArrayLibrary.Array_Contains` (`self.SecretsInRange`) Secret))
    (`KismetArrayLibrary.Array_Add` (`self.SecretsInRange`) Secret)
    (if (== (`KismetArrayLibrary.Array_Length` (`self.SecretsInRange`)) 1)
      (`/GGRadarSystem/UIs/WBP_Radar.Highlight Radar` (`self.WBP Radar`) true))))

(event `On Leave Secret Range`
  (params (Secret :type "/GGRadarSystem/Actors/AC_HighlightRadar_Base Object Reference"))
  ;[0 0 0] Event On Player Left Secret Range
  (if (`KismetArrayLibrary.Array_Contains` (`self.SecretsInRange`) Secret)
    (`KismetArrayLibrary.Array_RemoveItem` (`self.SecretsInRange`) Secret)
    (if (== (`KismetArrayLibrary.Array_Length` (`self.SecretsInRange`)) 0)
      (`/GGRadarSystem/UIs/WBP_Radar.Highlight Radar` (`self.WBP Radar`) false))))

(fn `Add Directions`
  (for _array_element (`self.Directions`)
    (`/GGRadarSystem/UIs/WBP_Radar.Add Direction` (`self.WBP Radar`) _array_element))
  (return))

(fn `Add Landmark To Radar`
  (params (Landmark :type "/GGRadarSystem/Actors/AC_Landmark_Base Object Reference"))
  (if (`KismetArrayLibrary.Array_Contains` (`self.Landmarks`) Landmark)
    (return)
    (else
      (`KismetArrayLibrary.Array_Add` (`self.Landmarks`) Landmark)
      (bind _wbp_radar (`self.WBP Radar`)
        (:`then`
          (`/GGRadarSystem/UIs/WBP_Radar.Add Landmark` _wbp_radar (`/GGRadarSystem/Actors/AC_Landmark_Base.Icon On Radar` Landmark))
          (return))
        (:`else`
          (return))))))

(fn `Add Landmarks`
  (bind _outactors (`GameplayStatics.GetAllActorsOfClass` "/GGRadarSystem/Actors/AC_Landmark_Base.AC_Landmark_Base_C"))
  (for _array_element _outactors
    (`self.Add Landmark To Radar` _array_element))
  (return))

(fn `Add Main Quest Marker`
  (params (`Main Quest Info` :type "/GGRadarSystem/Structures/FMarkerInfo Structure"))
  (locals (`New Main Quest Info` :type "/GGRadarSystem/Structures/FMarkerInfo Structure"))
  (set `local.New Main Quest Info` `Main Quest Info`)
  (`self.Remove Marker From Radar` (`self.Get Main Quest Info`))
  (`self.Set Main Quest Info` (`local.New Main Quest Info`))
  (`self.Add Marker To Radar` (`self.Main Quest Info`))
  (set `self.bHas Main Quest Selected` true)
  (`self.On Player Moved`))

(fn `Add Marker To Radar`
  (params (`Marker Info` :type "/GGRadarSystem/Structures/FMarkerInfo Structure"))
  (locals (`Local Marker Info` :type "/GGRadarSystem/Structures/FMarkerInfo Structure"))
  (bind _local_marker_info_type (break `/GGRadarSystem/Structures/FMarkerInfo` (`local.Local Marker Info`)))
  (bind _output_get (set `local.Local Marker Info` `Marker Info`))
  (`KismetArrayLibrary.Array_Add` (`self.Quest Markers`) _output_get)
  (bind _wbp_radar (`self.WBP Radar`)
    (:`then`
      (`/GGRadarSystem/UIs/WBP_Radar.Add Marker` _wbp_radar _local_marker_info_type)
      (return))
    (:`else`
      (return))))

(fn `Get Delta Clockwise`
  (params (A :type "Float (double-precision)") (B :type "Float (double-precision)") (bIsClockwise :type Boolean))
  (returns (Delta :type "Float (double-precision)"))
  (bind _returnvalue (mod A 360.0))
  (bind _returnvalue_2 (mod B 360.0))
  (bind _returnvalue_3 (mod B 360.0))
  (bind _returnvalue_4 (mod A 360.0))
  (if bIsClockwise
    (`/Engine/EditorBlueprintResources/StandardMacros.CompareFloat` _returnvalue_4 _returnvalue_3
      (:`>`
        (return (- 360.0 (- _returnvalue_4 _returnvalue_3))))
      (:`==`
        (return 0.0))
      (:`<`
        (return (- _returnvalue_3 _returnvalue_4))))
    (else
      (`/Engine/EditorBlueprintResources/StandardMacros.CompareFloat` _returnvalue _returnvalue_2
        (:`>`
          (return (- _returnvalue _returnvalue_2)))
        (:`==`
          (return 0.0))
        (:`<`
          (return (- 360.0 (- _returnvalue_2 _returnvalue))))))))

(fn `Get Main Quest Info`
  (returns (`Main Quest Info` :type "/GGRadarSystem/Structures/FMarkerInfo Structure"))
  (return (`self.Main Quest Info`)))

(fn `Has Main Quest Selected`
  (returns (`bHas Main Quest` :type Boolean))
  (return (`self.bHas Main Quest Selected`)))

(fn `Remove Main Quest Marker`
  (`self.Remove Marker From Radar` (`self.Get Main Quest Info`))
  (`self.Set Main Quest Info` (struct))
  (`self.On Player Moved`)
  (set `self.bHas Main Quest Selected` false))

(fn `Remove Marker From Radar`
  (params (Marker :type "/GGRadarSystem/Structures/FMarkerInfo Structure (by ref)"))
  (locals (`Marker Index` :type Integer :default 0))
  (bind _returnvalue (`KismetArrayLibrary.Array_Find` (`self.Quest Markers`) Marker))
  (if (>= _returnvalue 0)
    (set `local.Marker Index` _returnvalue)
    (`KismetArrayLibrary.Array_Remove` (`self.Quest Markers`) (`local.Marker Index`))
    (`Widget.RemoveFromParent` (`|GetArrayItem` (`/GGRadarSystem/UIs/WBP_Radar.Marker Widgets` (`self.WBP Radar`)) (`local.Marker Index`)))
    (`KismetArrayLibrary.Array_Remove` (`/GGRadarSystem/UIs/WBP_Radar.Marker Widgets` (`self.WBP Radar`)) (`local.Marker Index`))
    (return)
    (else
      (return))))

(fn `Rotation To Circle Degrees`
  (params (Input :type "Float (double-precision)"))
  (returns (Output :type "Float (double-precision)"))
  (return (`KismetMathLibrary.SelectFloat` (mod (+ Input 360.0) 360.0) Input (< Input 0.0))))

(fn `Rotations To Translation`
  (params (`Rotation A` :type "Rotator Structure") (`Rotation B` :type "Rotator Structure"))
  (returns (Translation :type "Vector2D Structure") (bIsClockwise :type Boolean) (bIsInRadarSight :type Boolean))
  (bind _output (`self.Rotation To Circle Degrees` (.yaw `Rotation B`)))
  (bind _output_2 (`self.Rotation To Circle Degrees` (.yaw `Rotation A`)))
  (bind _delta (`self.Get Delta Clockwise` _output_2 _output))
  (bind _delta_2 (`self.Get Delta Clockwise` _output_2 _output true))
  (bind _returnvalue (/ _delta_2 90.0))
  (bind _returnvalue_2 (/ _delta 90.0))
  (`/Engine/EditorBlueprintResources/StandardMacros.CompareFloat` _delta_2 _delta
    (:`>`
      (if (<= _returnvalue_2 1.0)
        (return (`KismetMathLibrary.MakeVector2D` (* (`KismetMathLibrary.Lerp` 0.0 (`self.Max Widget Translation`) _returnvalue_2) -1.0)) false true)
        (else
          (return (0.0 0.0) false false))))
    (:`==`
      _)
    (:`<`
      _))
  (if (<= _returnvalue 1.0)
    (return (`KismetMathLibrary.MakeVector2D` (`KismetMathLibrary.Lerp` 0.0 (`self.Max Widget Translation`) _returnvalue)) true true)
    (else
      (return (0.0 0.0) true false))))

(fn `Set Main Quest Info`
  (params (`Main Quest Info` :type "/GGRadarSystem/Structures/FMarkerInfo Structure"))
  (set `self.Main Quest Info` `Main Quest Info`)
  (return))

(fn `Toggle Visibility`
  (params (`Can Animate` :type Boolean))
  (`self.Set Radar Visibility` (not (`self.bIs Visible`)) `Can Animate`)
  (return))

(fn `Update Direction Widgets`
  (for (_array_element _array_index) (`/GGRadarSystem/UIs/WBP_Radar.Direction Widgets` (`self.WBP Radar`))
    (bind (_translation _bisclockwise _bisinradarsight) (`self.Rotations To Translation` (`SceneComponent.K2_GetComponentRotation` (`self.Camera Reference`)) (`KismetMathLibrary.MakeRotator` 0.0 0.0 (`KismetMathLibrary.Conv_IntToDouble` (`.WorldRotation_6_103771864B689D33859221B16F0B4DFD` (break `/GGRadarSystem/Structures/FWorldDirection` (`|GetArrayItem` (`self.Directions`) _array_index)))))))
    (if _bisinradarsight
      (`Widget.SetRenderTranslation` _array_element _translation)
      (bind _returnvalue (`Widget.IsVisible` _array_element))
      (if (not _returnvalue)
        (`Widget.SetVisibility` _array_element "SelfHitTestInvisible"))
      (elif _returnvalue
        (`Widget.SetVisibility` _array_element "Hidden")))))

(fn `Update Landmark Positions`
  (for (_array_element _array_index) (`/GGRadarSystem/UIs/WBP_Radar.Landmark Widgets` (`self.WBP Radar`))
    (bind (_translation _bisclockwise _bisinradarsight) (`self.Rotations To Translation` (`SceneComponent.K2_GetComponentRotation` (`self.Camera Reference`)) (`KismetMathLibrary.FindLookAtRotation` (`Actor.K2_GetActorLocation` (`self.Player Reference`)) (`Actor.K2_GetActorLocation` (`|GetArrayItem` (`self.Landmarks`) _array_index)))))
    (if _bisinradarsight
      (`Widget.SetRenderTranslation` _array_element _translation)
      (`Widget.SetVisibility` _array_element "SelfHitTestInvisible")
      (elif (`Widget.IsVisible` _array_element)
        (`Widget.SetVisibility` _array_element "Hidden"))))
  (return))

(fn `Update Marker Distances`
  (for (_array_element _array_index) (`/GGRadarSystem/UIs/WBP_Radar.Marker Widgets` (`self.WBP Radar`))
    (`/GGRadarSystem/UIs/WBP_Marker.Update Distance` _array_element (`KismetMathLibrary.Round` (/ (`KismetMathLibrary.VSize` (- (`KismetMathLibrary.MakeVector` (.x (`.Location_6_14B0A3084C4FE9B0D4A81B823637EBC7` (break `/GGRadarSystem/Structures/FMarkerInfo` (`|GetArrayItem` (`self.Quest Markers`) _array_index)))) (.y (`.Location_6_14B0A3084C4FE9B0D4A81B823637EBC7` (break `/GGRadarSystem/Structures/FMarkerInfo` (`|GetArrayItem` (`self.Quest Markers`) _array_index))))) (`KismetMathLibrary.MakeVector` (.x (`Actor.K2_GetActorLocation` (`self.Player Reference`))) (.y (`Actor.K2_GetActorLocation` (`self.Player Reference`)))))) (`self.Units Per Meter`)))))
  (return))

(fn `Update Marker Elevations`
  (bind _z (.z (`Actor.K2_GetActorLocation` (`self.Player Reference`))))
  (for (_array_element _array_index) (`/GGRadarSystem/UIs/WBP_Radar.Marker Widgets` (`self.WBP Radar`))
    (bind _z_2 (.z (`.Location_6_14B0A3084C4FE9B0D4A81B823637EBC7` (break `/GGRadarSystem/Structures/FMarkerInfo` (`|GetArrayItem` (`self.Quest Markers`) _array_index)))))
    (if (> _z_2 (+ _z (`self.Default Elevation Range`)))
      (`/GGRadarSystem/UIs/WBP_Marker.Set Arrow Direction` _array_element true)
      (`/GGRadarSystem/UIs/WBP_Marker.Set Arrow Visibility` _array_element true)
      (elif (< _z_2 (- _z (`self.Default Elevation Range`)))
        (`/GGRadarSystem/UIs/WBP_Marker.Set Arrow Direction` _array_element false)
        (`/GGRadarSystem/UIs/WBP_Marker.Set Arrow Visibility` _array_element true)
        (else
          (`/GGRadarSystem/UIs/WBP_Marker.Set Arrow Direction` _array_element false)
          (`/GGRadarSystem/UIs/WBP_Marker.Set Arrow Visibility` _array_element false)))))
  (return))

(fn `Update Marker Positions`
  (bind _max_widget_translation (`self.Max Widget Translation`))
  (for (_array_element _array_index) (`/GGRadarSystem/UIs/WBP_Radar.Marker Widgets` (`self.WBP Radar`))
    (if (`self.bAlwaysShowMarkers`)
      (bind (_translation _bisclockwise _bisinradarsight) (`self.Rotations To Translation` (`SceneComponent.K2_GetComponentRotation` (`self.Camera Reference`)) (`KismetMathLibrary.FindLookAtRotation` (`Actor.K2_GetActorLocation` (`self.Player Reference`)) (`.Location_6_14B0A3084C4FE9B0D4A81B823637EBC7` (break `/GGRadarSystem/Structures/FMarkerInfo` (`|GetArrayItem` (`self.Quest Markers`) _array_index))))))
      (`Widget.SetRenderTranslation` _array_element (select `bool` _bisinradarsight :`false` (`KismetMathLibrary.MakeVector2D` (select `bool` _bisclockwise :`false` (* _max_widget_translation -1.0) :`true` _max_widget_translation)) :`true` _translation))
      (elif _bisinradarsight
        (`Widget.SetRenderTranslation` _array_element _translation)
        (`Widget.SetVisibility` _array_element "SelfHitTestInvisible")
        (elif (`Widget.IsVisible` _array_element)
          (`Widget.SetVisibility` _array_element "Hidden")))))
  (return))